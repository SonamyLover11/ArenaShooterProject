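; Player character Blueprint handling movement, mouse look, jumping, dashing and firing.
; Input axes drive movement relative to control rotation and camera look, while Fire spawns a PlayerProj_BP projectile at the Arrow1 transform.
; Dash plays a sound and is gated by CanDash, reset on a short timer, but its launch velocity is zero.
; The dash Niagara effect and forward-velocity math are left unconnected.
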(event `InputAxis|MoveForward`
  (params (AxisValue :type "Float (single-precision)"))
  (bind (_returnvalue_roll _returnvalue_pitch _returnvalue_yaw) (`KismetMathLibrary.BreakRotator` (`self.GetControlRotation`)))
  ;[1 0.2986 0.6695 0.5] Movement
  (`self.AddMovementInput` (`KismetMathLibrary.GetForwardVector` (`KismetMathLibrary.MakeRotator` 0.0 0.0 _returnvalue_yaw)) AxisValue))

(event `InputAxis|MoveRight`
  (params (AxisValue :type "Float (single-precision)"))
  (bind (_returnvalue_roll _returnvalue_pitch _returnvalue_yaw) (`KismetMathLibrary.BreakRotator` (`self.GetControlRotation`)))
  ;[1 0.2986 0.6695 0.5] Movement
  (`self.AddMovementInput` (`KismetMathLibrary.GetRightVector` (`KismetMathLibrary.MakeRotator` _returnvalue_roll 0.0 _returnvalue_yaw)) AxisValue))

(event `InputAxis|LookUp`
  (params (AxisValue :type "Float (single-precision)"))
  ;[1 0.298 0.6706 0.502] Mouse Look
  (`self.AddControllerPitchInput` AxisValue))

(event `InputAction|Dash`
  (params (Key :type "Key Structure"))
  (:`Pressed`
    (if (`self.CanDash`)
      (`GameplayStatics.PlaySoundAtLocation` "/Game/Player/Dash_Cue.Dash_Cue" (`self.K2_GetActorLocation`) (struct) 1.0 1.0 0.0 null null null null)
      (`self.LaunchCharacter` (0.0 0.0 0.0))
      (set `self.CanDash` false)
      (`KismetSystemLibrary.K2_SetTimer` null "ResetDash" 0.5))))

(event `InputAction|Jump`
  (params (Key :type "Key Structure"))
  ;[1 0.2986 0.6695 0.5] Jump Event
  (:`Pressed`
    (`self.Jump`))
  (:`Released`
    (`self.StopJumping`)))

(event `InputAxis|Turn`
  (params (AxisValue :type "Float (single-precision)"))
  ;[1 0.298 0.6706 0.502] Mouse Look
  (`self.AddControllerYawInput` AxisValue))

(event `InputAction|Fire`
  (params (Key :type "Key Structure"))
  (:`Pressed`
    (`|SpawnActorFromClass` "/Game/Player/PlayerProj_BP.PlayerProj_BP_C" (`SceneComponent.K2_GetComponentToWorld` (`self.Arrow1`)) "Undefined" "MultiplyWithRoot" null null)))

(event `ResetDash`
  (set `self.CanDash` true))

(fn `UserConstructionScript`)