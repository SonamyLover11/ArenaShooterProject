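; AI controller Blueprint that starts the AI_BT behavior tree on BeginPlay.
; It has an AIPerception target-update event that checks whether the stimulus was successfully sensed, but neither branch acts on the result.
; Blackboard writes for LastKnownLocation and EnemyActor exist only as disconnected nodes, so perception does not feed the tree in this graph.
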(event `self.ReceiveBeginPlay`
  (`self.RunBehaviorTree` "/Game/AI/AI_BT.AI_BT"))

(event `self.AIPerception.OnTargetPerceptionUpdated`
  (params (Actor :type "Actor Object Reference") (Stimulus :type "AIStimulus Structure"))
  (if (`.bSuccessfullySensed` (break `AIStimulus` Stimulus))
    _))

(fn `UserConstructionScript`)