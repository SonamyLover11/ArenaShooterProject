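; Player character Blueprint with axis-driven movement relative to control rotation, mouse look, jumping and projectile firing.
; Fire spawns PlayerProj_BP at the Arrow1 transform with the character as owner.
; AnyDamage subtracts and prints Health, HealthBonus sets MaxHealth and refills it, and the CheckHP death branch is empty.
; Dash is unfinished: DoDash only tests CanDash, while the sound, launch, cooldown and Niagara nodes are disconnected.
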(event `InputAxis|MoveForward`
  (params (AxisValue :type "Float (single-precision)"))
  (bind (_returnvalue_roll _returnvalue_pitch _returnvalue_yaw) (`KismetMathLibrary.BreakRotator` (`self.GetControlRotation`)))
  ;[1 0.2986 0.6695 0.5] Movement
  (`self.AddMovementInput` (`KismetMathLibrary.GetForwardVector` (`KismetMathLibrary.MakeRotator` 0.0 0.0 _returnvalue_yaw)) AxisValue))

(event `InputAxis|MoveRight`
  (params (AxisValue :type "Float (single-precision)"))
  (bind (_returnvalue_roll _returnvalue_pitch _returnvalue_yaw) (`KismetMathLibrary.BreakRotator` (`self.GetControlRotation`)))
  ;[1 0.2986 0.6695 0.5] Movement
  (`self.AddMovementInput` (`KismetMathLibrary.GetRightVector` (`KismetMathLibrary.MakeRotator` _returnvalue_roll 0.0 _returnvalue_yaw)) AxisValue))

(event `InputAxis|LookUp`
  (params (AxisValue :type "Float (single-precision)"))
  ;[1 0.298 0.6706 0.502] Mouse Look
  (`self.AddControllerPitchInput` AxisValue))

(event `DoDash`
  (if (`self.CanDash`)
    _))

(event `InputAction|Dash`
  (params (Key :type "Key Structure")))

(event `InputAction|Jump`
  (params (Key :type "Key Structure"))
  ;[1 0.2986 0.6695 0.5] Jump Event
  (:`Pressed`
    (`self.Jump`))
  (:`Released`
    (`self.StopJumping`)))

(event `InputAxis|Turn`
  (params (AxisValue :type "Float (single-precision)"))
  ;[1 0.298 0.6706 0.502] Mouse Look
  (`self.AddControllerYawInput` AxisValue))

(event `ResetDash`
  (set `self.CanDash` true))

(event `InputAction|Fire`
  (params (Key :type "Key Structure"))
  ;[1 0.2986 0.6695 0.5] Fire event
  (:`Pressed`
    (`|SpawnActorFromClass` "/Game/Player/PlayerProj_BP.PlayerProj_BP_C" (`SceneComponent.K2_GetComponentToWorld` (`self.Arrow1`)) "Undefined" "MultiplyWithRoot" self null)))

(event `self.ReceiveAnyDamage`
  (params (Damage :type "Float (single-precision)") (DamageType :type "DamageType Object Reference") (InstigatedBy :type "Controller Object Reference") (DamageCauser :type "Actor Object Reference"))
  ;[1 0.2986 0.6695 0.5] Health and Damage
  (set `self.Damage Causer` DamageCauser)
  (set `self.Health` (- (`self.Health`) Damage))
  (`self.CheckHP`)
  (`KismetSystemLibrary.PrintString` (`KismetStringLibrary.Conv_DoubleToString` (`self.Health`))))

(event `CheckHP`
  ;[1 0.2986 0.6695 0.5] Health and Damage
  (if (<= (`self.Health`) 0.0)
    _))

(event `HealthBonus`
  (params (MaxHealth :type "Float (double-precision)"))
  ;[1 0.2986 0.6695 0.5] Health and Damage
  (bind _output_get (set `self.MaxHealth` MaxHealth))
  (set `self.Health` _output_get))

(fn `CheckHealth`)

(fn `UserConstructionScript`)